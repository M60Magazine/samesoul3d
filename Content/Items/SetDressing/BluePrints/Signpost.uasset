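; Signpost is a set-dressing Blueprint prop with four individually toggleable signs.
; Its construction script sets the visibility of each sign component from a matching boolean variable, without propagating to child components.
; The event graph holds only disabled placeholder events, so the prop adds no runtime logic.
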(event EventBeginPlay)

(event Collision|EventActorBeginOverlap
  (params (OtherActor :type Actor%20Object%20Reference)))

(event EventTick
  (params (DeltaSeconds :type Float%20%28single-precision%29)))

(fn ConstructionScript
  (Utilities|FlowControl|Sequence
    (:then_0
      (Rendering|SetVisibility (Variables|Default|GetSign1) (Variables|Default|GetSign1On) false))
    (:then_1
      (Rendering|SetVisibility (Variables|Default|GetSign2) (Variables|Default|GetSign2On) false))
    (:then_2
      (Rendering|SetVisibility (Variables|Default|GetSign3) (Variables|Default|GetSign3On) false))
    (:then_3
      (Rendering|SetVisibility (Variables|Default|GetSign4) (Variables|Default|GetSign4On) false))))